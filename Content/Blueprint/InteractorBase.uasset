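; InteractorBase is a base Blueprint for interactable actors, exposing Interaction and Hover events.
; Interaction runs InteractionAction only when the actor's origin, projected through player controller 0, lands inside the viewport bounds.
; Hover flips the MustHover flag on each call and passes it to DisplayObjectInteractibility.
; The action and hover responses are placeholders that only print debug strings.
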(event EventInteraction
  (params (Interactor :type Actor%20Object%20Reference))
  (CallFunction|InteractionTrigger))

(event EventHover
  (params (Hover :type Actor%20Object%20Reference))
  (bind _output_get (Variables|Default|SetmustHover (not (Variables|Default|GetmustHover))))
  (Development|PrintString (Utilities|String|Append (Utilities|String|ToString(Boolean) _output_get) " hover"))
  (CallFunction|DisplayObjectInteractibility))

(fn ConstructionScript)

(fn InteractionTrigger
  (bind _returnvalue (CallFunction|IsObjectonScreen))
  (if _returnvalue
    (CallFunction|InteractionAction)
    (else
      (Development|PrintString "Not On Screen !"))))

(fn IsObjectonScreen
  (bind _returnvalue (Viewport|GetViewportSize))
  (bind _returnvalue_2 (Transformation|GetActorLocation))
  (bind _returnvalue_3 (Game|GetPlayerController 0))
  (bind _screenlocation (Class|PlayerController|ProjectWorldLocationtoScreen _returnvalue_3 _returnvalue_2 false))
  (return (Math|Boolean|ANDBoolean (> (.x _screenlocation) 0.0) (> (.y _screenlocation) 0.0) (< (.x _screenlocation) (.x _returnvalue)) (< (.y _screenlocation) (.y _returnvalue)))))

(fn InteractionAction
  (Development|PrintString "ACTION"))

(fn DisplayObjectInteractibility
  (if (Variables|Default|GetmustHover)
    (Development|PrintString "Must launch Hover animation")
    (else
      (Development|PrintString "Must Stop Hover animation"))))
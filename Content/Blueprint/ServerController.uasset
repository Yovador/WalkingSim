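; ServerController is an actor that writes and reads billboard messages on a web server through the VaRest plugin.
; Writing sends a GET to the base Url with the billboard number and percent-encoded content in the query string.
; Reading clears CurrentBilboard and DataAvailable, fetches that billboard's JSON file, then fills the array from its "messages" field and sets DataAvailable once the asynchronous callback finishes.
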(event Custom|WriteCallback
  (params (Request :type Va%20Rest%20Request%20JSON%20Object%20Reference))
  (Development|PrintString "written"))

(event Custom|read
  (params (Request :type Va%20Rest%20Request%20JSON%20Object%20Reference))
  (Development|PrintString "ReadingJson")
  (for _array_element (Class|VaRestJsonObject|GetArrayField (Class|VaRestRequestJSON|GetResponseObject Request) "messages")
    (Development|PrintString "loop")
    (bind _returnvalue (Class|VaRestJsonValue|AsObject _array_element))
    (Utilities|Array|Add (Variables|Default|GetcurrentBilboard) _returnvalue))
  (Variables|Default|SetdataAvailable true))

(event EventAddMessagetoBilboardServer
  (params (bilboardNum :type Integer) (messageContent :type String))
  (bind _returnvalue (|VaRestSubsystem))
  (Development|PrintString "Hello")
  (bind _returnvalue_2 (Class|VaRestSubsystem|ConstructVaRestJsonObject _returnvalue))
  (bind _returnvalue_3 (Class|VaRestLibrary|PercentEncode messageContent))
  (Class|VaRestSubsystem|CallURL _returnvalue (Utilities|String|Append (Variables|Default|Geturl) "?" "bilboardNum=" (Utilities|String|ToString(Integer) bilboardNum) "&content=" _returnvalue_3) "GET" "x_www_form_urlencoded_url" _returnvalue_2 (delegate Custom|WriteCallback)))

(event EventReadMessagefromBilboardServer
  (params (bilboardNum :type Integer))
  (bind _returnvalue (|VaRestSubsystem))
  (Variables|Default|SetdataAvailable false)
  (Variables|Default|SetcurrentBilboard (Utilities|Array|MakeArray))
  (Development|PrintString "try read json")
  (bind _returnvalue_2 (Class|VaRestSubsystem|ConstructVaRestJsonObject _returnvalue))
  (Class|VaRestSubsystem|CallURL _returnvalue (Utilities|String|Append (Variables|Default|Geturl) "json/" "bilboard_" (Utilities|String|ToString(Integer) bilboardNum) ".json") "GET" "x_www_form_urlencoded_url" _returnvalue_2 (delegate Custom|read)))

(fn ConstructionScript)
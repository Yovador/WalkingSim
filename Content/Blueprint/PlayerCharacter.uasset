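; Player character with axis-driven look and movement, each switchable by events, that also posts a "player add" message to the ServerController billboard on BeginPlay.
; While movement is allowed, Tick moves it and diffs overlapping BPi_Interactable actors against the previous frame, sending HoverMessage on both entry and exit.
; Interact messages the first overlapping interactable, and beginning an overlap fires any BPi_EventTrigger actor.
; An unconnected example polls the server to read the billboard.
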(event Collision|EventActorBeginOverlap
  (params (OtherActor :type Actor%20Object%20Reference))
  ;[0.04167 0.04167 0.04167] Trigger Event
  (if (Utilities|DoesObjectImplementInterface OtherActor "/Game/Blueprint/Interface/BPi_EventTrigger.BPi_EventTrigger_C")
    (Class|BPiEventTrigger|TriggerEvent(Message) OtherActor)))

(event EventBeginPlay
  (Development|PrintString "BeginPlay")
  (bind _outactors (Actor|GetAllActorsOfClass "/Game/Blueprint/ServerController.ServerController_C"))
  (Development|PrintString "get all actor of class server")
  (Default|AddMessagetoBilboardServer (Utilities|Array|Get(acopy) _outactors) 0 "player add"))

(event EventChangePlayerCanLook
  (params (newCanLook :type Boolean))
  (Variables|Default|SetcanLook newCanLook))

(event EventTick
  (params (DeltaSeconds :type Float%20%28single-precision%29))
  ;[0.05208 0.05208 0.05208] Movement
  (if (Variables|Default|GetcanMove)
    (Pawn|Input|AddMovementInput (Math|Vector|Normalize (+ (* (Transformation|GetActorForwardVector) (Input|AxisValues|GetForwardAxis)) (* (Transformation|GetActorRightVector) (Input|AxisValues|GetSideAxis)))) (Variables|Default|GetmoveSpeed) false)
    ;[0.09896 0.03301 0.02165] Hover Behavior
    ;;[0.08854 0.08854 0.08854] Get all interactor currently in range
    (bind _array_element (Utilities|Array|ForEachLoopwithBreak (Collision|GetOverlappingActors (Variables|Collision|GetCapsuleComponent) 0 :!class /Script/Engine.PrimitiveComponent))
      (:LoopBody
        (if (Utilities|DoesObjectImplementInterface _array_element "/Game/Blueprint/Interface/BPi_Interactable.BPi_Interactable_C")
          ;;;[0.08854 0.08854 0.08854] Store all interactor of this frame
          (Utilities|Array|Add (Variables|Default|GetcurrentInteractor) _array_element)
          ;;;[0.08854 0.08854 0.08854] If Interactor is new, activate hover
          (if (not (Utilities|Array|ContainsItem (Variables|Default|GetpreviousInteractor) _array_element))
            (Class|BPiInteractable|Hover(Message) _array_element))))
      (:Completed
        ;;[0.08854 0.08854 0.08854] If one interactor who were in range previously isn't anymore, deactivate hover
        (for _array_element_2 (Variables|Default|GetpreviousInteractor)
          (if (not (Utilities|Array|ContainsItem (Variables|Default|GetcurrentInteractor) _array_element_2))
            (Class|BPiInteractable|Hover(Message) _array_element_2)))
        ;;[0.08854 0.08854 0.08854] Update previous interactor, and empty current interactor
        (Variables|Default|SetpreviousInteractor (Variables|Default|GetcurrentInteractor))
        (Variables|Default|SetcurrentInteractor (Utilities|Array|MakeArray 0))))))

(event EventChangePlayerCanMove
  (params (newCanMove :type Boolean))
  (Variables|Default|SetcanMove newCanMove))

(event Input|ActionEvents|InputActionInteract
  (params (Key :type Key%20Structure :default "None"))
  ;[0.09896 0.09896 0.09896] Interact
  (:Pressed
    (Development|PrintString "Press Interact")
    (bind _array_element (Utilities|Array|ForEachLoopwithBreak (Collision|GetOverlappingActors (Variables|Collision|GetCapsuleComponent) 0 :!class /Script/Engine.PrimitiveComponent) :!label _label)
      (:LoopBody
        (Development|PrintString (Utilities|GetObjectName _array_element))
        (if (Utilities|DoesObjectImplementInterface _array_element "/Game/Blueprint/Interface/BPi_Interactable.BPi_Interactable_C")
          (Class|BPiInteractable|Interaction(Message) _array_element)
          (goto _label Break))))))

(event Input|AxisEvents|InputAxisLookHorizontal
  (params (AxisValue :type Float%20%28single-precision%29))
  ;[0.09896 0.09896 0.09896] LookingAround
  (if (Variables|Default|GetcanLook)
    (Pawn|Input|AddControllerYawInput (* AxisValue (Variables|Default|GetmouseSensibility)))))

(event Input|AxisEvents|InputAxisLookVertical
  (params (AxisValue :type Float%20%28single-precision%29))
  ;[0.09896 0.09896 0.09896] LookingAround
  (if (Variables|Default|GetcanLook)
    (Pawn|Input|AddControllerPitchInput (* AxisValue -1.0 (Variables|Default|GetmouseSensibility)))))

(fn ConstructionScript
  (bind _array (Utilities|Array|MakeArray 0))
  (Variables|Default|SetpreviousInteractor _array)
  (Variables|Default|SetcurrentInteractor _array))
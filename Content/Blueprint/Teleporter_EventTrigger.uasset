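; Event trigger child Blueprint that teleports the first player's character to a target actor.
; Its EventAction override calls the parent, then moves the character to TeleportTarget's location while keeping the actor's rotation.
; It clears EventAlreadyTrigger, presumably so the trigger can fire again, then sets the controller's rotation to the Rotation variable.
; Debug strings print the teleport and the flag state.
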(event EventBeginPlay)

(event Collision|EventActorBeginOverlap
  (params (OtherActor :type Actor%20Object%20Reference)))

(event EventTick
  (params (DeltaSeconds :type Float%20%28single-precision%29)))

(fn ConstructionScript
  (|CallParentFunction))

(fn EventAction
  (bind _returnvalue (Game|GetPlayerCharacter 0))
  (|CallParentFunction)
  (Development|PrintString "Teleport")
  (Transformation|Teleport _returnvalue (Transformation|GetActorLocation (Variables|Default|GetTeleportTarget)) (Transformation|GetActorRotation _returnvalue))
  (bind _output_get (Variables|Default|SeteventAlreadyTrigger false))
  (Development|PrintString (Utilities|String|ToString(Boolean) _output_get))
  (Pawn|SetControlRotation (Pawn|GetController (Game|GetPlayerCharacter 0)) (Variables|Default|Getrotation)))
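; AlarmLight is a pulsing alarm light actor that drives a light, an emissive-style material and audio together.
; The construction script creates a dynamic material instance from a base material, applies the configured color and assigns it to the cube mesh.
; On BeginPlay, the AlarmTime timeline's Intensity track sets light brightness, scaled by AlarmIntensity, along with the material's Intensity parameter and the audio volume.
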(event EventBeginPlay
  (bind _intensity (Timeline|AlarmTime Play)
    (:Update
      (Rendering|Components|Light|SetIntensity (Variables|Default|GetLightComponent) (* _intensity (Variables|Default|GetAlarmIntensity)))
      (Rendering|Material|SetScalarParameterValue (Variables|Default|GetMaterial) "Intensity" _intensity :!class /Script/Engine.MaterialInstanceDynamic)
      (Audio|Components|Audio|SetVolumeMultiplier (Variables|Default|GetAudio) _intensity :!class /Script/Engine.AudioComponent))))

(fn ConstructionScript
  (bind _returnvalue (Rendering|Material|CreateDynamicMaterialInstance (Variables|Default|GetBaseMat) "None" "None" :!class /Script/Engine.KismetMaterialLibrary))
  (bind _output_get (Variables|Default|SetMaterial _returnvalue))
  (Rendering|Material|SetScalarParameterValue _output_get "Intensity" 1.0 :!class /Script/Engine.MaterialInstanceDynamic)
  (Rendering|Material|SetVectorParameterValue _output_get "Color" (Math|Conversions|ToLinearColor(Color) (Variables|Default|GetColor)) :!class /Script/Engine.MaterialInstanceDynamic)
  (Rendering|Material|SetMaterial (Variables|Default|GetCube) 0 _output_get))
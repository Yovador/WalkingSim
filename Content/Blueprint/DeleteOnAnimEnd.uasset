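; Actor that removes itself after its skeletal mesh animation starts playing, optionally chaining into a follow-up actor.
; BeginPlay applies the configured hidden state, and Tick unhides the actor once the mesh is playing.
; After a configurable delay it optionally sends LaunchActionMessage to a target object, then destroys its attached actors and itself.
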(event EventTick
  (params (DeltaSeconds :type Float%20%28single-precision%29))
  (if (Audio|Components|Audio|IsPlaying (Variables|SkeletalMeshActor|GetSkeletalMeshComponent))
    (Rendering|SetActorHiddenInGame false)
    (Utilities|FlowControl|Delay (Variables|Default|GetwaitTime))
    (if (Variables|Default|GethasFollowUpAnim)
      (Class|BPiTriggerResponder|LaunchAction(Message) (Variables|Default|GetObjectToTrigger)))
    (for _array_element (Actor|GetAttachedActors true)
      (Actor|DestroyActor _array_element))
    (Actor|DestroyActor)))

(event EventBeginPlay
  (Rendering|SetActorHiddenInGame (Variables|Default|GetisHidden)))

(fn ConstructionScript)
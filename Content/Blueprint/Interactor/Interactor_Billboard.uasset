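; Interactable billboard actor that shows a prompt on hover and toggles a text widget when interacted with.
; Each Hover call flips a flag that creates or removes the prompt widget.
; Interaction proceeds only if the actor's projected position lies inside the viewport, then removes the prompt.
; A FlipFlop alternates between opening the widget with cursor and game pause, and removing it without restoring either.
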(event EventInteraction
  (CallFunction|InteractionTrigger))

(event EventHover
  (Variables|Default|SetmustHover (not (Variables|Default|GetmustHover)))
  (CallFunction|DisplayObjectInteractibility))

(fn ConstructionScript)

(fn InteractionTrigger
  (bind _returnvalue (CallFunction|IsObjectonScreen))
  (if _returnvalue
    (Widget|RemovefromParent (Variables|Default|GetInteractPrompt))
    (CallFunction|InteractionAction)
    (else
      (Development|PrintString "Not On Screen !"))))

(fn IsObjectonScreen
  (bind _returnvalue (Viewport|GetViewportSize))
  (bind _returnvalue_2 (Transformation|GetActorLocation))
  (bind _returnvalue_3 (Game|GetPlayerController 0))
  (bind _screenlocation (Class|PlayerController|ProjectWorldLocationtoScreen _returnvalue_3 _returnvalue_2 false))
  (return (Math|Boolean|ANDBoolean (> (.x _screenlocation) 0.0) (> (.y _screenlocation) 0.0) (< (.x _screenlocation) (.x _returnvalue)) (< (.y _screenlocation) (.y _returnvalue)))))

(fn InteractionAction
  (Widget|RemovefromParent (Variables|Default|GetInteractPrompt))
  (Utilities|FlowControl|FlipFlop
    (:A
      (bind _returnvalue (UserInterface|CreateWidget "/Game/Blueprint/Widgets/PlayerInputUI/InputsTextWidget.InputsTextWidget_C"))
      (UserInterface|Viewport|AddtoViewport _returnvalue 0)
      (Variables|/Script/Engine.PlayerController|SetbShowMouseCursor (Game|GetPlayerController 0) true)
      (Game|SetGamePaused true))
    (:B
      (Widget|RemovefromParent _returnvalue))))

(fn DisplayObjectInteractibility
  (if (Variables|Default|GetmustHover)
    (bind _returnvalue (UserInterface|CreateWidget "/Game/Blueprint/Widgets/InteractUI/InteractPrompt.InteractPrompt_C"))
    (bind _output_get (Variables|Default|SetInteractPrompt _returnvalue))
    (UserInterface|Viewport|AddtoViewport _output_get 0)
    (else
      (Widget|RemovefromParent (Variables|Default|GetInteractPrompt)))))